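; Player ball character, stored in the Obsolete folder, that moves and turns a Ball component together with its SpringArm.
; Each Tick matches the arm's yaw to the ball's, adds the Turn input, then copies the result back to the ball.
; MoveForward and MoveRight inputs shift both components along relative X and Y by fixed steps, without delta-time scaling or regard to yaw.
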(event `self.ReceiveTick`
  (params (DeltaSeconds :type "Float (single-precision)"))
  (bind _ball (`self.ball`))
  (bind _springarm (`self.SpringArm`))
  (bind _springarm_2 (`self.SpringArm`))
  (bind (_relativerotation_roll _relativerotation_pitch) (`KismetMathLibrary.BreakRotator` (`SceneComponent.RelativeRotation` _ball)))
  (bind (_relativerotation_roll_2 _relativerotation_pitch_2 _relativerotation_yaw) (`KismetMathLibrary.BreakRotator` (`SceneComponent.RelativeRotation` (`self.SpringArm`))))
  (bind (_relativerotation_roll_3 _relativerotation_pitch_3) (`KismetMathLibrary.BreakRotator` (`SceneComponent.RelativeRotation` _springarm_2)))
  (bind (_relativerotation_roll_4 _relativerotation_pitch_4 _relativerotation_yaw_2) (`KismetMathLibrary.BreakRotator` (`SceneComponent.RelativeRotation` (`self.ball`))))
  (bind (_relativerotation_roll_5 _relativerotation_pitch_5 _relativerotation_yaw_3) (`KismetMathLibrary.BreakRotator` (`SceneComponent.RelativeRotation` _springarm)))
  ;[1 1 1] camera tweaks
  (`SceneComponent.K2_SetRelativeRotation` _springarm_2 (`KismetMathLibrary.MakeRotator` _relativerotation_roll_3 _relativerotation_pitch_3 _relativerotation_yaw_2) false false)
  (`SceneComponent.K2_SetRelativeRotation` _springarm (`KismetMathLibrary.MakeRotator` _relativerotation_roll_5 _relativerotation_pitch_5 (+ _relativerotation_yaw_3 (`self.GetInputAxisValue`))) false false)
  (`SceneComponent.K2_SetRelativeRotation` _ball (`KismetMathLibrary.MakeRotator` _relativerotation_roll _relativerotation_pitch _relativerotation_yaw) false false))

(event `InputAxis|MoveForward`
  (params (AxisValue :type "Float (single-precision)"))
  (`self.MoveForward` (`self.ball`) AxisValue)
  (`self.MoveForward` (`self.SpringArm`) AxisValue))

(event `InputAction|enablefan`
  (params (Key :type "Key Structure")))

(event `InputAxis|MoveRight`
  (params (AxisValue :type "Float (single-precision)"))
  (`self.MoveRight` (`self.ball`) AxisValue)
  (`self.MoveRight` (`self.SpringArm`) AxisValue))

(fn `MoveForward`
  (params (`object to move` :type "SceneComponent Object Reference") (`input value` :type "Float (double-precision)"))
  (bind (_relativelocation_x _relativelocation_y _relativelocation_z) (`KismetMathLibrary.BreakVector` (`SceneComponent.RelativeLocation` `object to move`)))
  (`SceneComponent.K2_SetRelativeLocation` `object to move` (`KismetMathLibrary.MakeVector` (+ _relativelocation_x (* 5 `input value`)) _relativelocation_y _relativelocation_z) false false))

(fn `MoveRight`
  (params (`object to move` :type "SceneComponent Object Reference") (`input value` :type "Float (double-precision)"))
  (bind (_relativelocation_x _relativelocation_y _relativelocation_z) (`KismetMathLibrary.BreakVector` (`SceneComponent.RelativeLocation` `object to move`)))
  (`SceneComponent.K2_SetRelativeLocation` `object to move` (`KismetMathLibrary.MakeVector` _relativelocation_x (+ _relativelocation_y (* 5 `input value`)) _relativelocation_z) false false))

(fn `UserConstructionScript`)