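; BP_MainBall is the player's ball pawn, handling startup possession, fan input and the pause menu.
; On BeginPlay, player controller 0 possesses it and StartingCamera becomes the current camera.
; Holding the enablefan input switches the fan on through the FanBall game mode, and releasing it switches it off.
; Pause creates WBP_PauseMenu and switches to UI-only input, without pausing the game itself in this graph.
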(event `self.ReceiveBeginPlay`
  ;[1 1 1] BeginPlay
  (`Controller.Possess` (`GameplayStatics.GetPlayerController` 0) self)
  (`/Game/Blueprints/CoreBlueprints/BP_StaticCamera.SetThisCameraAsCurrent` (`self.StartingCamera`)))

(event `InputAction|enablefan`
  (params (Key :type "Key Structure"))
  (bind _fanballgamemode (`/Game/FanBallBPLCore.GetFanBallGameMOde` self))
  ;[1 1 1] EnableFAn
  (:`Pressed`
    (`/Game/Blueprints/CoreBlueprints/BP_FanBallGameMode.togglefan` _fanballgamemode true))
  (:`Released`
    (`/Game/Blueprints/CoreBlueprints/BP_FanBallGameMode.togglefan` _fanballgamemode false)))

(event `InputAction|Pause`
  (params (Key :type "Key Structure"))
  ;[1 1 1] Pause
  (:`Pressed`
    (bind _returnvalue (`|CreateWidget` "/Game/Blueprints/Widgets/WBP_PauseMenu.WBP_PauseMenu_C"))
    (`UserWidget.AddToViewport` _returnvalue 0)
    (`WidgetBlueprintLibrary.SetInputMode_UIOnlyEx` (`GameplayStatics.GetPlayerController` 0) _returnvalue)))

(fn `UserConstructionScript`)