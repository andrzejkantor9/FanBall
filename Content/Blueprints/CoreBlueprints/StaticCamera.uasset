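; StaticCamera is a fixed camera for the fan-and-ball game that takes over the player's view when the MainBall enters its area.
; Two trigger components detect the ball and switch the view target to this camera, recording it as current on FanBallGameMOde.
; If the fan is on at that moment, it also calls the game mode's fan toggle.
; Debug prints report camera switches and Jump presses.
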(event `InputAction|Jump`
  (params (Key :type "Key Structure"))
  (:`Pressed`
    (`KismetSystemLibrary.PrintString` "jump")))

(event `self.EnterThisCamera.OnComponentBeginOverlap`
  (params (OverlappedComponent :type "PrimitiveComponent Object Reference") (OtherActor :type "Actor Object Reference") (OtherComp :type "PrimitiveComponent Object Reference") (OtherBodyIndex :type Integer) (bFromSweep :type Boolean) (SweepResult :type "HitResult Structure (by ref)"))
  ;[1 1 1] start this camera
  (if (`KismetMathLibrary.ClassIsChildOf` (`GameplayStatics.GetObjectClass` OtherActor) "/Game/Blueprints/CoreBlueprints/MainBall.MainBall_C")
    (`self.SetThisCameraAsCurrent` :!label _label)
    (if (`/Game/Blueprints/CoreBlueprints/BP_FanBallGameMode.FanOn` (`/Game/FanBallBPLCore.GetFanBallGameMOde` self))
      (`/Game/Blueprints/CoreBlueprints/BP_FanBallGameMode.togglefan` (`/Game/FanBallBPLCore.GetFanBallGameMOde` self) true))))

(event `self.EnterThisCamera1.OnComponentBeginOverlap`
  (params (OverlappedComponent :type "PrimitiveComponent Object Reference") (OtherActor :type "Actor Object Reference") (OtherComp :type "PrimitiveComponent Object Reference") (OtherBodyIndex :type Integer) (bFromSweep :type Boolean) (SweepResult :type "HitResult Structure (by ref)"))
  ;[1 1 1] start this camera
  (if (`KismetMathLibrary.ClassIsChildOf` (`GameplayStatics.GetObjectClass` OtherActor) "/Game/Blueprints/CoreBlueprints/MainBall.MainBall_C")
    (goto _label)))

(fn `SetThisCameraAsCurrent`
  (`PlayerController.SetViewTargetWithBlend` (`GameplayStatics.GetPlayerController` 0) self 0.0 "VTBlend_Linear" 0.0 false)
  (set `/Game/Blueprints/CoreBlueprints/BP_FanBallGameMode.currentcamera` self (`/Game/FanBallBPLCore.GetFanBallGameMOde` self))
  (`KismetSystemLibrary.PrintString` (`KismetStringLibrary.Concat_StrStr` "Use camera: " (`KismetSystemLibrary.GetDisplayName` self))))

(fn `UserConstructionScript`)