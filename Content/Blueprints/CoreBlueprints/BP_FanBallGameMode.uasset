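; Game mode for FanBall that manages the game's menus and switches the fan tied to the current camera.
; On BeginPlay it shows the pause menu with UI-only input focus, and ShowWinScreen does the same for the win screen.
; Togglefan enables or disables the fan referenced by Currentcamera and records the state in FanOn, while DisableActiveFans switches that fan off without updating the flag.
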(event `self.ReceiveBeginPlay`
  (bind _returnvalue (`|CreateWidget` "/Game/Blueprints/Widgets/WBP_PauseMenu.WBP_PauseMenu_C"))
  (`UserWidget.AddToViewport` _returnvalue 0)
  (`WidgetBlueprintLibrary.SetInputMode_UIOnlyEx` (`GameplayStatics.GetPlayerController` 0) _returnvalue))

(fn `DisableActiveFans`
  (`/Game/Blueprints/PhysicsObjects/fan.EnableFan` (`/Game/Blueprints/CoreBlueprints/BP_StaticCamera.fantouse` (`self.currentcamera`)) false))

(fn `ShowWinScreen`
  (bind _returnvalue (`|CreateWidget` "/Game/Blueprints/Widgets/WBP_WinScreen.WBP_WinScreen_C"))
  (`UserWidget.AddToViewport` _returnvalue 0)
  (`WidgetBlueprintLibrary.SetInputMode_UIOnlyEx` (`GameplayStatics.GetPlayerController` 0) _returnvalue))

(fn `togglefan`
  (params (on :type Boolean))
  (`/Game/Blueprints/PhysicsObjects/fan.EnableFan` (`/Game/Blueprints/CoreBlueprints/BP_StaticCamera.fantouse` (`self.currentcamera`)) on)
  (set `self.FanOn` on))

(fn `UserConstructionScript`)